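; BP_MasterDoor is a double door that the player can open only after collecting all keys.
; Overlapping Box1 enables input, and leaving it disables input.
; Interact asks SwordCharacter whether all keys are collected, then toggles two timelines that yaw each door leaf open or closed and plays a gate sound.
; Timeline updates also disable StaticMesh collision; debug prints report the key check.
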(event `InputAction|Interact`
  (params (Key :type "Key Structure"))
  ;[1 1 1] Check if all keys collected or not
  (:`Pressed`
    (bind _assword_character (cast `/Game/FirstPersonBP/Blueprints/SwordCharacter` (`GameplayStatics.GetPlayerCharacter` 0)))
    (bind _all_keys_collected__ (`/Game/FirstPersonBP/Blueprints/SwordCharacter.All Keys Collected` _assword_character))
    (if _all_keys_collected__
      (`KismetSystemLibrary.PrintString` "All Keys Collected. Open Master Door")
      (`|ExecutionSequence`
        (:`then_0`
          ;[1 1 1] Open / Close Left Door
          (if (`self.Is Open Left`)
            (set `self.Is Open Left` false)
            (bind (_direction _yaw) (`Timeline|Door yaw` :!via `Reverse` :!label _label)
              (:`Update`
                (`SceneComponent.K2_SetRelativeRotation` (`self.Left Door 1`) (`KismetMathLibrary.MakeRotator` 0.0 0.0 _yaw) false false)
                (`PrimitiveComponent.SetCollisionEnabled` (`self.StaticMesh`) "NoCollision" :!label _label_2)))
            (else
              (set `self.Is Open Left` true)
              (goto _label))))
        (:`then_1`
          ;[1 1 1] Open / Close Right Door
          (if (`self.Is Open Right`)
            (set `self.Is Open Right` false)
            (bind (_direction_2 _yaw_2) (`Timeline|Timeline_0` :!via `Reverse` :!label _label_3)
              (:`Update`
                (`SceneComponent.K2_SetRelativeRotation` (`self.Left Door 2`) (`KismetMathLibrary.MakeRotator` 0.0 0.0 _yaw_2) false false)
                (goto _label_2)))
            (else
              (set `self.Is Open Right` true)
              (goto _label_3))))
        (:`then_2`
          (`GameplayStatics.PlaySoundAtLocation` "/Game/Sounds/MetalGateOpen.MetalGateOpen" (`self.K2_GetActorLocation`) (struct) 1.0 1.0 0.0 null null null)))
      (else
        (`KismetSystemLibrary.PrintString` "NOT all keys collected. Cannot open door.")))))

(event `self.Box1.OnComponentBeginOverlap`
  (params (OverlappedComponent :type "PrimitiveComponent Object Reference") (OtherActor :type "Actor Object Reference") (OtherComp :type "PrimitiveComponent Object Reference") (OtherBodyIndex :type Integer) (bFromSweep :type Boolean) (SweepResult :type "HitResult Structure (by ref)"))
  ;[1 1 1] enable/ disable input
  (if (== OtherActor (`GameplayStatics.GetPlayerCharacter` 0))
    (`self.EnableInput` (`GameplayStatics.GetPlayerController` 0))))

(event `self.Box1.OnComponentEndOverlap`
  (params (OverlappedComponent :type "PrimitiveComponent Object Reference") (OtherActor :type "Actor Object Reference") (OtherComp :type "PrimitiveComponent Object Reference") (OtherBodyIndex :type Integer))
  ;[1 1 1] enable/ disable input
  (if (== (`GameplayStatics.GetPlayerCharacter` 0) OtherActor)
    (`self.DisableInput` (`GameplayStatics.GetPlayerController` 0))))

(fn `UserConstructionScript`
  (`parent.UserConstructionScript`))