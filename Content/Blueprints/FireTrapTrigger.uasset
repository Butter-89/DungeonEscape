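; Trigger actor that switches a linked BP_DragonFireTrap on while the SwordCharacter overlaps it.
; On overlap it casts its TarpFiring reference to the trap, sets IsActive and launches a fireball with a zero vector immediately.
; A looped Delay on the trap's RateOfFire repeats the launch while IsActive holds.
; End overlap clears IsActive, so the loop stops after the pending delay.
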(event `self.ReceiveActorBeginOverlap`
  (params (OtherActor :type "Actor Object Reference"))
  (cast `/Game/FirstPersonBP/Blueprints/SwordCharacter` OtherActor)
  (bind _asbp_dragon_fire_trap (cast `/Game/Blueprints/BP_DragonFireTrap` (`self.TarpFiring`)))
  (set `/Game/Blueprints/BP_DragonFireTrap.IsActive` true _asbp_dragon_fire_trap)
  (`/Game/Blueprints/BP_DragonFireTrap.LauchFireBall` _asbp_dragon_fire_trap (0.0 0.0 0.0) :!label _label)
  (`KismetSystemLibrary.Delay` (`/Game/Blueprints/BP_DragonFireTrap.RateOfFire` _asbp_dragon_fire_trap))
  (if (`/Game/Blueprints/BP_DragonFireTrap.IsActive` _asbp_dragon_fire_trap)
    (goto _label)))

(event `self.ReceiveActorEndOverlap`
  (params (OtherActor :type "Actor Object Reference"))
  (cast `/Game/FirstPersonBP/Blueprints/SwordCharacter` OtherActor)
  (bind _asbp_dragon_fire_trap (cast `/Game/Blueprints/BP_DragonFireTrap` (`self.TarpFiring`)))
  (set `/Game/Blueprints/BP_DragonFireTrap.IsActive` false _asbp_dragon_fire_trap))

(fn `UserConstructionScript`)