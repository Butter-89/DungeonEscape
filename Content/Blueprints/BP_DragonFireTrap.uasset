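; BP_DragonFireTrap is a trap actor that launches a fireball at the player with a dragon roar sound.
; LauchFireBall spawns a FireBall at LaunchStart, aims its projectile velocity at player 0's current location scaled by Speed, and sets ToPlayer.
; The PlayerLocation input is ignored.
; The event graph's delayed launch is disconnected, so nothing inside this Blueprint triggers firing.
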(event `self.ReceiveBeginPlay`)

(fn `LauchFireBall`
  (params (PlayerLocation :type "Vector Structure"))
  (bind _returnvalue (`|SpawnActorFromClass` "/Game/Blueprints/EnemyAI/Boss/FireBall.FireBall_C" (`SceneComponent.K2_GetComponentToWorld` (`self.LaunchStart`)) "AdjustIfPossibleButAlwaysSpawn" "OverrideRootScale" null null))
  (`GameplayStatics.PlaySoundAtLocation` "/Game/Sounds/442964__qubodup__dragon-roar.442964__qubodup__dragon-roar" (`self.K2_GetActorLocation`) (struct) 1.0 1.0 0.0 null null null)
  (bind _output_get (set `MovementComponent.Velocity` (* (`KismetMathLibrary.GetDirectionUnitVector` (`SceneComponent.K2_GetComponentLocation` (`self.LaunchStart`)) (`self.K2_GetActorLocation` (`GameplayStatics.GetPlayerCharacter` 0))) (`self.Speed`)) (`self.GetComponentByClass` _returnvalue "/Script/Engine.ProjectileMovementComponent")))
  (set `/Game/Blueprints/EnemyAI/Boss/FireBall.ToPlayer` true _returnvalue))

(fn `UserConstructionScript`)