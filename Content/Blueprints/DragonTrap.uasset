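; Dragon trap enemy that growls, attacks the player in range with fireballs, and drops a golden key when destroyed.
; Overlap events track the SwordCharacter, while Tick turns the dragon's yaw toward the player and fires at intervals using a CanFire gate and delay.
; Fireballs are aimed at the player and flagged ToPlayer.
; An unflagged fireball hitting the capsule sets off two timed explosions before the dragon destroys itself.
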(event `self.ReceiveBeginPlay`
  (bind _returnvalue (`GameplayStatics.SpawnSoundAtLocation` "/Game/Sounds/427414__mega-x-stream__dinosaur-dragon-growls.427414__mega-x-stream__dinosaur-dragon-growls" (`self.K2_GetActorLocation`) (struct) 1.0 1.0 0.0 null null))
  (set `self.DragonSound` _returnvalue))

(event `self.ReceiveDestroyed`
  ;[1 1 1] Drop key
  (`|SpawnActorFromClass` "/Game/FirstPersonBP/Blueprints/BP_GoldenKey.BP_GoldenKey_C" (`KismetMathLibrary.Conv_VectorToTransform` (`SceneComponent.K2_GetComponentLocation` (`self.KeyDropPosition`))) "AdjustIfPossibleButAlwaysSpawn" "OverrideRootScale" null null)
  (`AudioComponent.Stop` (`self.DragonSound`)))

(event `self.ReceiveTick`
  (params (DeltaSeconds :type "Float (single-precision)"))
  ;[1 1 1] Look at Player when entering the range
  (if (`self.PlayerInRange`)
    (`self.K2_SetActorRotation` (`KismetMathLibrary.MakeRotator` 0.0 0.0 (.yaw (`KismetMathLibrary.FindLookAtRotation` (`self.K2_GetActorLocation` self) (`self.K2_GetActorLocation` (`GameplayStatics.GetPlayerCharacter` 0))))))
    (if (`self.CanFire`)
      (set `self.CanFire` false)
      (`self.LaunchFireBalls_Comp`)
      (`KismetSystemLibrary.RetriggerableDelay` (`self.FireInterval`))
      (set `self.CanFire` true)
      (set `self.AttackAnimation` true)
      (`KismetSystemLibrary.Delay` 0.2)
      (set `self.AttackAnimation` false))))

(event `self.ReceiveActorBeginOverlap`
  (params (OtherActor :type "Actor Object Reference"))
  (bind _returnvalue (`self.K2_GetActorLocation`))
  (bind _capsulecomponent (`self.CapsuleComponent`))
  ;[1 1 1] Detect if player is in range
  (cast `/Game/FirstPersonBP/Blueprints/SwordCharacter` OtherActor
    (:`then`
      (set `self.PlayerInRange` true))
    (:`CastFailed`
      (bind (_outactors _returnvalue_2) (`KismetSystemLibrary.ComponentOverlapActors` _capsulecomponent (`SceneComponent.K2_GetComponentToWorld` _capsulecomponent) (`|MakeArray` "ObjectTypeQuery7" "ObjectTypeQuery2" :!type "EObjectTypeQuery Enum") "/Game/Blueprints/EnemyAI/Boss/FireBall.FireBall_C"))
      (if _returnvalue_2
        (bind _asfire_ball (cast `/Game/Blueprints/EnemyAI/Boss/FireBall` OtherActor))
        (if (not (`/Game/Blueprints/EnemyAI/Boss/FireBall.ToPlayer` _asfire_ball))
          (`self.K2_DestroyActor` OtherActor)
          (`GameplayStatics.SpawnEmitterAtLocation` "/Game/StarterContent/Particles/P_Explosion.P_Explosion" _returnvalue (struct) (10.0 10.0 10.0))
          (`GameplayStatics.PlaySoundAtLocation` "/Game/Sounds/FireExplosion.FireExplosion" (`self.K2_GetActorLocation`) (struct) 1.0 1.0 0.0 null null null)
          (`KismetSystemLibrary.Delay` 1.5)
          (`GameplayStatics.SpawnEmitterAtLocation` "/Game/StarterContent/Particles/P_Explosion.P_Explosion" _returnvalue (struct) (10.0 10.0 10.0))
          (`GameplayStatics.PlaySoundAtLocation` "/Game/Sounds/FireExplosion.FireExplosion" (`self.K2_GetActorLocation`) (struct) 1.0 1.0 0.0 null null null)
          (`KismetSystemLibrary.Delay` 1.0)
          (`self.K2_DestroyActor`))))))

(event `self.ReceiveActorEndOverlap`
  (params (OtherActor :type "Actor Object Reference"))
  ;[1 1 1] Detect if player is in range
  (cast `/Game/FirstPersonBP/Blueprints/SwordCharacter` OtherActor)
  (set `self.PlayerInRange` false))

(event `self.SphereCollider.OnComponentBeginOverlap`
  (params (OverlappedComponent :type "PrimitiveComponent Object Reference") (OtherActor :type "Actor Object Reference") (OtherComp :type "PrimitiveComponent Object Reference") (OtherBodyIndex :type Integer) (bFromSweep :type Boolean) (SweepResult :type "HitResult Structure (by ref)")))

(fn `DecreaseHP`)

(fn `LaunchFireBalls`
  (params (PlaceToStart :type "Actor Object Reference"))
  (bind _returnvalue (* (`KismetMathLibrary.GetDirectionUnitVector` (`SceneComponent.K2_GetComponentLocation` (`self.LaunchStart`)) (`self.K2_GetActorLocation` (`GameplayStatics.GetPlayerCharacter` 0))) (`self.FireballSpeed`)))
  (bind _returnvalue_2 (`|SpawnActorFromClass` "/Game/Blueprints/EnemyAI/Boss/FireBall.FireBall_C" (`SceneComponent.K2_GetComponentToWorld` (`Actor.RootComponent` PlaceToStart)) "AdjustIfPossibleButAlwaysSpawn" "OverrideRootScale" null null))
  (bind _asfire_ball (cast `/Game/Blueprints/EnemyAI/Boss/FireBall` _returnvalue_2))
  (`KismetSystemLibrary.PrintString` (`KismetStringLibrary.Conv_VectorToString` _returnvalue))
  (set `MovementComponent.Velocity` _returnvalue (`self.GetComponentByClass` _asfire_ball "/Script/Engine.ProjectileMovementComponent"))
  (set `/Game/Blueprints/EnemyAI/Boss/FireBall.ToPlayer` true _asfire_ball))

(fn `LaunchFireBalls_Comp`
  (bind _returnvalue (* (`KismetMathLibrary.GetDirectionUnitVector` (`SceneComponent.K2_GetComponentLocation` (`self.LaunchStart`)) (`self.K2_GetActorLocation` (`GameplayStatics.GetPlayerCharacter` 0))) (`self.FireballSpeed`)))
  (bind _returnvalue_2 (`|SpawnActorFromClass` "/Game/Blueprints/EnemyAI/Boss/FireBall.FireBall_C" (`SceneComponent.K2_GetComponentToWorld` (`self.LaunchStart`)) "AdjustIfPossibleButAlwaysSpawn" "OverrideRootScale" null null))
  (`GameplayStatics.PlaySoundAtLocation` "/Game/Sounds/442964__qubodup__dragon-roar.442964__qubodup__dragon-roar" (`self.K2_GetActorLocation`) (struct) 1.0 1.0 0.0 null null null)
  (bind _asfire_ball (cast `/Game/Blueprints/EnemyAI/Boss/FireBall` _returnvalue_2))
  (`KismetSystemLibrary.PrintString` (`KismetStringLibrary.Conv_VectorToString` _returnvalue))
  (set `MovementComponent.Velocity` _returnvalue (`self.GetComponentByClass` _asfire_ball "/Script/Engine.ProjectileMovementComponent"))
  (set `/Game/Blueprints/EnemyAI/Boss/FireBall.ToPlayer` true _asfire_ball))

(fn `UpdateWalkSpeed`
  (params (NewWalkSpeed :type "Float (double-precision)"))
  (set `CharacterMovementComponent.MaxWalkSpeed` NewWalkSpeed (`self.CharacterMovement`)))

(fn `UserConstructionScript`)