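; BP_Door is an interactable door that the player opens and closes with the Interact input.
; A box overlap enables input on the actor while the player character is inside and disables it on exit.
; Each press flips IsOpen and plays or reverses the DoorYawModification timeline, which drives the static mesh's relative yaw to swing the door.
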(event `self.Box1.OnComponentBeginOverlap`
  (params (OverlappedComponent :type "PrimitiveComponent Object Reference") (OtherActor :type "Actor Object Reference") (OtherComp :type "PrimitiveComponent Object Reference") (OtherBodyIndex :type Integer) (bFromSweep :type Boolean) (SweepResult :type "HitResult Structure (by ref)"))
  ;[1 1 1] Detects the collission with the player and enablesw door opening on pressing 'E'
  ;;[1 1 1] Enable Input
  (if (== OtherActor (`GameplayStatics.GetPlayerCharacter` 0))
    (`self.EnableInput` (`GameplayStatics.GetPlayerController` 0))))

(event `InputAction|Interact`
  (params (Key :type "Key Structure"))
  ;[1 1 1] Detects the collission with the player and enablesw door opening on pressing 'E'
  ;;[1 1 1] Open/Close on Interact
  (:`Pressed`
    (if (`self.IsOpen`)
      (set `self.IsOpen` false)
      (bind (_direction _door_yaw_modification) (`Timeline|Door Yaw Modification` :!via `Reverse` :!label _label)
        (:`Update`
          (`SceneComponent.K2_SetRelativeRotation` (`self.StaticMesh`) (`KismetMathLibrary.MakeRotator` 0.0 0.0 _door_yaw_modification) false false)))
      (else
        (set `self.IsOpen` true)
        (goto _label)))))

(event `self.Box1.OnComponentEndOverlap`
  (params (OverlappedComponent :type "PrimitiveComponent Object Reference") (OtherActor :type "Actor Object Reference") (OtherComp :type "PrimitiveComponent Object Reference") (OtherBodyIndex :type Integer))
  ;[1 1 1] Detects the collission with the player and enablesw door opening on pressing 'E'
  ;;[1 1 1] Enable Input
  (if (== (`GameplayStatics.GetPlayerCharacter` 0) OtherActor)
    (`self.DisableInput` (`GameplayStatics.GetPlayerController` 0))))

(fn `UserConstructionScript`)